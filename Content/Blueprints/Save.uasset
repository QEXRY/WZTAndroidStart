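; Save helper Blueprint that persists the game's ranking list through a BP_MySave SaveGame object in a fixed slot.
; LoadRanking loads the slot and returns its RankingList, stopping with no result if the cast to BP_MySave fails.
; SaveGame appends a RankMessage to the loaded list and writes it back, creating a new BP_MySave when none loads.
; Entries are appended without sorting or trimming.
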(fn LoadRanking
  (bind _returnvalue (SaveGame|LoadGamefromSlot "111"))
  (bind _asbp_my_save (Utilities|Casting|CastToBP_MySave _returnvalue))
  (return (Variables|/Game/Blueprints/BP_MySave.BP_MySave_C|GetRankingList _asbp_my_save)))

(fn SaveGame
  (params (RankMessage :type S%20Rank%20Bar%20Structure))
  (bind _returnvalue (SaveGame|LoadGamefromSlot "111"))
  (bind _asbp_my_save (Utilities|Casting|CastToBP_MySave _returnvalue)
    (:then
      (Utilities|Array|Add (Variables|/Game/Blueprints/BP_MySave.BP_MySave_C|GetRankingList _asbp_my_save) RankMessage)
      (SaveGame|SaveGametoSlot _asbp_my_save "111"))
    (:CastFailed
      (bind _returnvalue_2 (SaveGame|CreateSaveGameObject "/Game/Blueprints/BP_MySave.BP_MySave_C"))
      (Utilities|Array|Add (Variables|/Game/Blueprints/BP_MySave.BP_MySave_C|GetRankingList _returnvalue_2) RankMessage)
      (SaveGame|SaveGametoSlot _returnvalue_2 "111"))))